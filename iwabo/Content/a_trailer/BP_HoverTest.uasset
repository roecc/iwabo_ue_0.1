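; BP_HoverTest is a test actor that highlights its static meshes while the mouse cursor hovers over its Mesh component.
; The Construction Script and BeginPlay both assign the MeshShape variable to Mesh.
; Cursor-over events toggle Render Custom Depth on every StaticMeshComponent of the actor, the usual hook for post-process outlines.
; Clicking Mesh only prints a debug string.
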(event OnBeginCursorOver(Mesh)
  (params (TouchedComponent :type Primitive%20Component%20Object%20Reference))
  (for _array_element (Actor|GetComponentsByClass "/Script/Engine.StaticMeshComponent")
    (Rendering|SetRenderCustomDepth _array_element true)))

(event OnEndCursorOver(Mesh)
  (params (TouchedComponent :type Primitive%20Component%20Object%20Reference))
  (for _array_element (Actor|GetComponentsByClass "/Script/Engine.StaticMeshComponent")
    (Rendering|SetRenderCustomDepth _array_element false)))

(event OnClicked(Mesh)
  (params (TouchedComponent :type Primitive%20Component%20Object%20Reference) (ButtonPressed :type Key%20Structure :default "None"))
  (Development|PrintString "Clicked!"))

(event EventBeginPlay
  (Components|StaticMesh|SetStaticMesh (Variables|Default|GetMesh) (Variables|Default|GetMeshShape)))

(event Collision|EventActorBeginOverlap
  (params (OtherActor :type Actor%20Object%20Reference)))

(event EventTick
  (params (DeltaSeconds :type Float%20%28single-precision%29)))

(fn ConstructionScript
  (Components|StaticMesh|SetStaticMesh (Variables|Default|GetMesh) (Variables|Default|GetMeshShape)))