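; Interactable trailer spot that presents rations, keeping those in its InteractRange in line with the game instance's available stock.
; Interact switches to a temporary camera and enables input, and IA_Move closes the conversation, restoring range collision and the camera.
; On BeginPlay and NewTurn, after a short delay, it tallies overlapping rations by type, collects the excess, then destroys them in a second pass.
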(event Custom|NewTurn
  (Utilities|FlowControl|Delay 0.3)
  (Variables|Default|SetRationsOnTable (Utilities|Map|MakeMap "NewEnumerator0" 0 "NewEnumerator1" 0 "NewEnumerator2" 0))
  (bind _asbp_game_instance (Utilities|Casting|CastToBP_GameInstance (Game|GetGameInstance)))
  (for _array_element (Collision|GetOverlappingActors (Variables|Default|GetInteractRange) 0 :!class /Script/Engine.PrimitiveComponent)
    (bind _asbp_ration_base (Utilities|Casting|CastToBP_Ration_Base _array_element))
    (if (> (+ (.Value (Utilities|Map|Find (Variables|Default|GetRationsOnTable) (Variables|/Game/Interactables/DayMechanics/FoodTable/BP_Ration_Base.BP_Ration_Base_C|GetRationType _asbp_ration_base))) 1) (.Value (Utilities|Map|Find (Variables|/Game/GameManagement/BP_GameInstance.BP_GameInstance_C|GetAvailableRations _asbp_game_instance) (Variables|/Game/Interactables/DayMechanics/FoodTable/BP_Ration_Base.BP_Ration_Base_C|GetRationType _asbp_ration_base))))
      (Utilities|Array|Add (Variables|Default|GetDEBUG_ToDestroy) _array_element)
      (else
        (Utilities|Map|Add (Variables|Default|GetRationsOnTable) (Variables|/Game/Interactables/DayMechanics/FoodTable/BP_Ration_Base.BP_Ration_Base_C|GetRationType _asbp_ration_base) (+ (.Value (Utilities|Map|Find (Variables|Default|GetRationsOnTable) (Variables|/Game/Interactables/DayMechanics/FoodTable/BP_Ration_Base.BP_Ration_Base_C|GetRationType _asbp_ration_base))) 1)))))
  ;[0.08854 0.08854 0.08854] Destroy All Excess
  (for _array_element_2 (Variables|Default|GetDEBUG_ToDestroy)
    (Utilities|IsValid _array_element_2
      (:Is%20Valid
        (Actor|DestroyActor _array_element_2)))))

(event Input|EnhancedActionEvents|EnhancedInputActionIA_Move
  (params (ActionValue :type Vector%202D%20Structure) (ElapsedSeconds :type Float%20%28double-precision%29) (TriggeredSeconds :type Float%20%28double-precision%29) (InputAction :type Input%20Action%20Object%20Reference :default "/Game/ThirdPerson/Input/Actions/IA_Move.IA_Move"))
  (CallFunction|ConversationClosed))

(event EventBeginPlay
  (Utilities|FlowControl|Delay 0.3)
  (Variables|Default|SetRationsOnTable (Utilities|Map|MakeMap "NewEnumerator0" 0 "NewEnumerator1" 0 "NewEnumerator2" 0))
  (bind _asbp_game_instance (Utilities|Casting|CastToBP_GameInstance (Game|GetGameInstance)))
  (for _array_element (Collision|GetOverlappingActors (Variables|Default|GetInteractRange) 0 :!class /Script/Engine.PrimitiveComponent)
    (bind _asbp_ration_base (Utilities|Casting|CastToBP_Ration_Base _array_element))
    (if (> (+ (.Value (Utilities|Map|Find (Variables|Default|GetRationsOnTable) (Variables|/Game/Interactables/DayMechanics/FoodTable/BP_Ration_Base.BP_Ration_Base_C|GetRationType _asbp_ration_base))) 1) (.Value (Utilities|Map|Find (Variables|/Game/GameManagement/BP_GameInstance.BP_GameInstance_C|GetAvailableRations _asbp_game_instance) (Variables|/Game/Interactables/DayMechanics/FoodTable/BP_Ration_Base.BP_Ration_Base_C|GetRationType _asbp_ration_base))))
      (Utilities|Array|Add (Variables|Default|GetDEBUG_ToDestroy) _array_element)
      (else
        (Utilities|Map|Add (Variables|Default|GetRationsOnTable) (Variables|/Game/Interactables/DayMechanics/FoodTable/BP_Ration_Base.BP_Ration_Base_C|GetRationType _asbp_ration_base) (+ (.Value (Utilities|Map|Find (Variables|Default|GetRationsOnTable) (Variables|/Game/Interactables/DayMechanics/FoodTable/BP_Ration_Base.BP_Ration_Base_C|GetRationType _asbp_ration_base))) 1)))))
  ;[0.08854 0.08854 0.08854] Destroy All Excess
  (for _array_element_2 (Variables|Default|GetDEBUG_ToDestroy)
    (Utilities|IsValid _array_element_2
      (:Is%20Valid
        (Actor|DestroyActor _array_element_2)))))

(event EventInteract
  (params (Instigator :type Actor%20Object%20Reference))
  (Collision|SetCollisionEnabled (Variables|Default|GetInteractRange) "NoCollision")
  (Variables|Default|SetInteractInstigator Instigator)
  (Input|EnableInput (Game|GetPlayerController 0))
  (Utilities|FlowControl|Delay 0.2)
  (Input|SetInputModeGameOnly (Game|GetPlayerController 0) false)
  (Default|SwitchtoTmp (Variables|Default|GetAC_TmpCam) (Variables|Default|GetInteractInstigator)))

(event EventConversationClosed
  (Collision|SetCollisionEnabled (Variables|Default|GetInteractRange) "QueryOnly")
  (Input|DisableInput (Game|GetPlayerController 0))
  (Class|BPIInteractable|ConversationClosed(Message) (Variables|Default|GetInteractInstigator))
  (Default|SwitchBack (Variables|Default|GetAC_TmpCam)))

(fn ConstructionScript
  (|CallParentFunction))