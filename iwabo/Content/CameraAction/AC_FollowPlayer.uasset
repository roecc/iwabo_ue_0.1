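; Actor component for a CameraActor that makes the camera follow the player character along Y and Z, keeping its own X.
; On BeginPlay for cameras auto-activating for player 0, or on ActivateCam, it registers itself as the character's DebugCam, sets InvertControls and captures the starting offset.
; While active, Tick repositions the camera from the player's location plus that offset.
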(event Custom|ActivateCam
  (bind _returnvalue (Game|GetPlayerCharacter 0))
  (bind _asbp_third_person_character (Utilities|Casting|CastToBP_ThirdPersonCharacter _returnvalue))
  (Variables|/Game/ThirdPerson/Blueprints/BP_ThirdPersonCharacter.BP_ThirdPersonCharacter_C|SetdebugCam _asbp_third_person_character (stale EventBeginPlay _ascamera_actor))
  (Variables|/Game/ThirdPerson/Blueprints/BP_ThirdPersonCharacter.BP_ThirdPersonCharacter_C|SetInvertControls _asbp_third_person_character 1)
  (bind _output_get (Variables|Default|SetTarget _returnvalue))
  (Variables|Default|SetOffset (- (Transformation|GetActorLocation (Components|GetOwner)) (Transformation|GetActorLocation _output_get)))
  (Variables|Default|SetbIsActiveCam? true))

(event EventBeginPlay
  (bind _returnvalue (Game|GetPlayerCharacter 0))
  (bind _ascamera_actor (Utilities|Casting|CastToCameraActor (Components|GetOwner)))
  (if (== (Class|CameraActor|GetAutoActivatePlayerIndex _ascamera_actor) 0)
    (bind _asbp_third_person_character (Utilities|Casting|CastToBP_ThirdPersonCharacter _returnvalue))
    (Variables|/Game/ThirdPerson/Blueprints/BP_ThirdPersonCharacter.BP_ThirdPersonCharacter_C|SetdebugCam _asbp_third_person_character _ascamera_actor)
    (Variables|/Game/ThirdPerson/Blueprints/BP_ThirdPersonCharacter.BP_ThirdPersonCharacter_C|SetInvertControls _asbp_third_person_character 1)
    (bind _output_get (Variables|Default|SetTarget _returnvalue))
    (Variables|Default|SetOffset (- (Transformation|GetActorLocation (Components|GetOwner)) (Transformation|GetActorLocation _output_get)))
    (Variables|Default|SetbIsActiveCam? true)))

(event EventTick
  (params (DeltaSeconds :type Float%20%28single-precision%29))
  (bind _returnvalue (Components|GetOwner))
  (bind _target (Variables|Default|GetTarget))
  (bind _offset (Variables|Default|GetOffset))
  (bind _returnvalue_2 (Transformation|GetActorLocation _target))
  (bind _returnvalue_3 (+ _returnvalue_2 _offset))
  (if (Variables|Default|GetbIsActiveCam?)
    (Utilities|IsValid _target
      (:Is%20Valid
        (Transformation|SetActorLocation _returnvalue (Math|Vector|MakeVector (.x (Transformation|GetActorLocation _returnvalue)) (.y _returnvalue_3) (.z _returnvalue_3)) false false)))))