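; Switchable level camera that registers itself as the third-person character's current camera and blends the player's view to it on activation.
; While active, Tick either aims from a fixed position, orbits a pivot to track the player's angle and height, or follows along X or Y plus height.
; In non-fixed modes, mouse movement past a screen threshold yaws the arm or slides the camera sideways, easing near its limit.
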(event Custom|ActivateCam
  (bind _returnvalue (Game|GetPlayerCharacter 0))
  (bind _asbp_third_person_character (Utilities|Casting|CastToBP_ThirdPersonCharacter _returnvalue))
  (Variables|/Game/ThirdPerson/Blueprints/BP_ThirdPersonCharacter.BP_ThirdPersonCharacter_C|SetCurrentCam _asbp_third_person_character self)
  (bind _output_get (Variables|Default|SetTarget _returnvalue))
  (Utilities|FlowControl|Sequence
    (:then_0
      (Utilities|FlowControl|DoOnce false
        (:Completed
          (Variables|Default|SetOffset (- (Transformation|GetActorLocation) (Transformation|GetActorLocation _output_get))))))
    (:then_1
      _))
  (Variables|Default|SetbIsActiveCam? true)
  (Game|Player|SetViewTargetwithBlend (Game|GetPlayerController 0) self 1.0 "VTBlend_Linear" 0.0 false))

(event Custom|DeactivateCam
  (Variables|Default|SetbIsActiveCam? false))

(event EventBeginPlay
  (if (Variables|Default|GetbIsActiveCam?)
    (CallFunction|ActivateCam)))

(event EventTick
  (params (DeltaSeconds :type Float%20%28single-precision%29))
  (bind _returnvalue (Transformation|GetActorTransform))
  (bind _returnvalue_2 (Transformation|GetActorLocation))
  (bind _returnvalue_3 (Game|GetPlayerCharacter 0))
  (bind _target (Variables|Default|GetTarget))
  (bind _offset (Variables|Default|GetOffset))
  (bind _returnvalue_4 (Transformation|GetActorLocation _target))
  (bind _returnvalue_5 (+ _returnvalue_4 _offset))
  (if (not (Variables|Default|GetbNoMoveCam?))
    (if (Variables|Default|GetbIsActiveCam?)
      (if (Variables|Default|GetbIsFixedPos?)
        (Transformation|SetActorRotation (Math|Rotator|FindLookatRotation (Transformation|GetWorldLocation (Variables|Default|GetCamera)) (Transformation|GetActorLocation (Variables|Default|GetTarget))))
        (else
          (|GetRelativeMousePos)
          (if (Variables|Default|GetbIsRotary?)
            ;[1 1 1] Rotate
            (Transformation|SetActorRotation (Math|Rotator|MakeRotator 0.0 0.0 (- (.yaw (Math|Rotator|FindLookatRotation (.location (Transformation|GetActorTransform)) (.location (Transformation|GetActorTransform _returnvalue_3)))) -1.8e+02)))
            (Transformation|SetActorLocation (Math|Vector|MakeVector (.x (.location _returnvalue)) (.y (.location _returnvalue)) (.z (.location (Transformation|GetActorTransform _returnvalue_3)))) false false)
            (bind _returnvalue_6 (CallFunction|CheckThreshold))
            (if _returnvalue_6
              (bind _returnvalue_7 (|CamOffsetY_2 (* (.x (Variables|Default|GetmousePos)) -1.0) (Variables|Default|Getl2mSpeed) (Variables|Default|Getl2mMax))
                (:OutputPin
                  (Transformation|AddRelativeRotation (Variables|Default|GetCamArmFixpoint) (Math|Rotator|MakeRotator 0.0 0.0 _returnvalue_7) false false))))
            (else
              (if (Variables|Default|GetbFollowX?)
                ;[1 1 1] fixed x
                (Transformation|SetActorLocation (Math|Vector|MakeVector (.x _returnvalue_5) (.y _returnvalue_2) (.z _returnvalue_5)) false false)
                (else
                  (Transformation|SetActorLocation (Math|Vector|MakeVector (.x _returnvalue_2) (.y (+ _returnvalue_4 "")) (.z _returnvalue_5)) false false)))
              (bind _returnvalue_8 (CallFunction|CheckThreshold))
              (if _returnvalue_8
                (bind (_camera _returnvalue_9) (|CamOffsetY (.x (Variables|Default|GetmousePos)) (Variables|Default|Getl2mSpeed) (Variables|Default|Getl2mMax) (Variables|Default|GetCamera))
                  (:OutputPin
                    (Transformation|AddRelativeLocation _camera (Math|Vector|MakeVector 0.0 _returnvalue_9 0.0) false false)))))))))))

(fn ConstructionScript)

(fn CheckThreshold
  (bind _mousepos (Variables|Default|GetmousePos))
  (if (> (.x _mousepos) (Variables|Default|Getl2mThreshhold))
    (return true)
    (elif (< (.x _mousepos) (* (Variables|Default|Getl2mThreshhold) -1.0))
      (return true)
      (else
        (return false)))))