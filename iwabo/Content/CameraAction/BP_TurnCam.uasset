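; BP_TurnCam is a camera actor that stays at its horizontal position and turns to track the player character.
; On BeginPlay it registers itself as the DebugCam on the player's BP_ThirdPersonCharacter.
; Each Tick it sets its yaw from a look-at rotation toward the player and matches the player's height, keeping its own X and Y.
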(event EventBeginPlay
  (bind _asbp_third_person_character (Utilities|Casting|CastToBP_ThirdPersonCharacter (Game|GetPlayerCharacter 0)))
  (Variables|/Game/ThirdPerson/Blueprints/BP_ThirdPersonCharacter.BP_ThirdPersonCharacter_C|SetdebugCam _asbp_third_person_character self))

(event Collision|EventActorBeginOverlap
  (params (OtherActor :type Actor%20Object%20Reference)))

(event EventTick
  (params (DeltaSeconds :type Float%20%28single-precision%29))
  (bind _returnvalue (Transformation|GetActorTransform))
  (bind _returnvalue_2 (Game|GetPlayerCharacter 0))
  (Transformation|SetActorRotation (Math|Rotator|MakeRotator 0.0 0.0 (.yaw (Math|Rotator|FindLookatRotation (.location (Transformation|GetActorTransform)) (.location (Transformation|GetActorTransform _returnvalue_2))))))
  (Transformation|SetActorLocation (Math|Vector|MakeVector (.x (.location _returnvalue)) (.y (.location _returnvalue)) (.z (.location (Transformation|GetActorTransform _returnvalue_2)))) false false))

(fn ConstructionScript)