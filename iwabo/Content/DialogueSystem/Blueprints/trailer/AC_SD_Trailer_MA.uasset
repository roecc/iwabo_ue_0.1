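; Actor component for the DialogueSystem trailer that starts a cinematic in response to direction cues.
; It overrides TakeDirection, calls the parent, and on "shot1" destroys any existing sequence player actor, then creates and plays the LS_BunkerDialogue Level Sequence.
; The new sequence actor is stored in CurrentPlayer for later cleanup.
; A disconnected fragment that would move the owning NPC_Base to a random location never runs.
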(event EventBeginPlay)

(event EventTick
  (params (DeltaSeconds :type Float%20%28single-precision%29)))

(fn TakeDirection
  (params (Direction :type String))
  (|CallParentFunction Direction)
  (if (Utilities|Enum|Equal(Enum) Direction "shot1")
    (if (Utilities|IsValid (Variables|Default|GetCurrentPlayer))
      (Actor|DestroyActor (Variables|Default|GetCurrentPlayer)))
    (bind (_outactor _returnvalue) (Sequencer|Player|CreateLevelSequencePlayer "/Game/DialogueSystem/Blueprints/trailer/LS_BunkerDialogue.LS_BunkerDialogue"))
    (Variables|Default|SetCurrentPlayer _outactor)
    (Sequencer|Player|Play _returnvalue :!class /Script/MovieScene.MovieSceneSequencePlayer)))