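; Dialogue actor component that runs a branching conversation through WB_Dialogue, here one short Mary-Ann and Daryl exchange.
; Each choice is saved in DialogueProgress, then the tree replays from the top, passing visited nodes until a new one updates the widget.
; Macros wrap lines, options and voice sounds, with speakers resolved from CharacterData.
; An unconnected data-table helper reads pipe-delimited localized lines and prints options for debugging.
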(fn OpenConversation
  (bind _returnvalue (UserInterface|CreateWidget "/Game/DialogueSystem/UI/WB_Dialogue.WB_Dialogue_C" 0 self))
  (bind _output_get (Variables|Default|SetDialogueWidget _returnvalue))
  (UserInterface|Viewport|AddtoViewport _output_get 0)
  (CallFunction|ProgressDialogue))

(fn CloseConversation
  (Widget|RemovefromParent (Variables|Default|GetDialogueWidget))
  (Class|BPIInteractable|ConversationClosed(Message) (Components|GetOwner)))

(fn ProgressDialogue
  (Variables|Default|SetDialogueIndex -1)
  (CallFunction|Dialogue))

(fn Dialogue
  (|Choice_4_2 "Hm?" "NewEnumerator0" "Uhm, Daryl?"
    (:1
      (CallFunction|ClearDialogueProgress)
      (CallFunction|CloseConversation))))

(fn AddDialogue
  (params (Speaker :type DA%20Character%20Data%20Object%20Reference) (Dialogue :type Text) (OptionsText :type Array%20of%20Texts) (OptionDelay :type Float%20%28double-precision%29) (ResponseTime :type Float%20%28double-precision%29))
  (bind _dialogueprogress (Variables|Default|GetDialogueProgress))
  (bind _dialogueindex (Variables|Default|GetDialogueIndex))
  (bind (_value _returnvalue) (Utilities|Map|Find _dialogueprogress _dialogueindex))
  (Math|Integer|IncrementInt (Variables|Default|GetDialogueIndex)
    (:%20%20
      (if _returnvalue
        (return "NewEnumerator0" _value)
        (else
          (Default|UpdateDialogueText (Variables|Default|GetDialogueWidget) (Variables|Default|GetDialogueIndex) Speaker Dialogue OptionsText OptionDelay ResponseTime)
          (return "NewEnumerator1" 0))))))

(fn UpdateSelectedOption
  (params (ProgressIndex :type Integer%20%28by%20ref%29) (OptionIndex :type Integer%20%28by%20ref%29))
  (Utilities|Map|Add (Variables|Default|GetDialogueProgress) ProgressIndex OptionIndex)
  (CallFunction|ProgressDialogue))

(fn ClearDialogueProgress
  (Utilities|Map|Clear (Variables|Default|GetDialogueProgress)))

(fn RemoveDialogueProgress
  (params (ProgressSteps :type Integer))
  (for _index (range 0 ProgressSteps)
    (Utilities|Map|Remove (Variables|Default|GetDialogueProgress) (- (Variables|Default|GetDialogueIndex) _index))))

(fn SetDialogueTreeIndex
  (params (DialogueTreeIndex :type Integer))
  (Variables|Default|SetDialogueTreeIndex DialogueTreeIndex)
  (CallFunction|ClearDialogueProgress))

(fn FetchBlockfromDT
  (params (Table :type Data%20Table%20Object%20Reference) (RowName :type Name))
  (bind _returnvalue (Utilities|GetDataTableRow Table RowName)
    (:then
      (bind _returnvalue_2 (CallFunction|GetLang (.joined_line (Utilities|Struct|BreakS_DT_Dialogue _returnvalue))))
      (|DebugLogLine_2 _returnvalue_2 :!label _label
        (:OutputPin
          (bind _index (Utilities|FlowControl|ForLoopwithBreak 0 10 :!label _label_2)
            (:LoopBody
              (bind _returnvalue_3 (Utilities|GetDataTableRow Table (Utilities|String|StringToName (Utilities|String|Append (Utilities|String|ToString(Name) RowName) "_" (Utilities|String|ToString(Integer) _index))))
                (:then
                  (bind _returnvalue_4 (CallFunction|GetLang (.joined_line (Utilities|Struct|BreakS_DT_Dialogue _returnvalue_3))))
                  (|DebugLogOptions_2 _index _returnvalue_4))
                (:RowNotFound
                  (if (not (== _index 0)) ; Test beyond Silent option
                    (goto _label_2 Break)))))
            (:Completed
              (return (Utilities|Text|ToText(String) _returnvalue_2)))))))
    (:RowNotFound
      (goto _label not%20found))))

(fn GetLang
  (params (SourceString :type String))
  (bind _returnvalue (Utilities|String|ParseIntoArray SourceString "|" false))
  (bind _language (Variables|Default|GetLanguage))
  ;[1 1 1] Continue only if the array has at least one element.
  (if (> (Utilities|Array|Length _returnvalue) _language)
    (LocalVariables|SetOutput (Utilities|Array|Get(acopy) _returnvalue _language)))
  (return (LocalVariables|GetOutput)))

(fn DatafromEnum
  (params (InputPin :type Enum_Character%20Enum :default "NewEnumerator0"))
  (Utilities|FlowControl|Sequence
    (:then_0
      (switch Utilities|FlowControl|Switch|SwitchonEnum_Character InputPin
        (:NewEnumerator0
          (LocalVariables|SetIndex 0))
        (:NewEnumerator1
          (LocalVariables|SetIndex 1))
        (:NewEnumerator2
          (LocalVariables|SetIndex 2))
        (:NewEnumerator3
          (LocalVariables|SetIndex 3))))
    (:then_1
      (return (Utilities|Array|Get(acopy) (Variables|Default|GetCharacterData) (LocalVariables|GetIndex))))))