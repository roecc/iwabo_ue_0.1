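; Base dialogue component that runs data-table-driven conversations through a WB_Dialogue widget.
; Each block is fetched by row name, picks its language from a pipe-delimited string and gathers options from suffixed rows, with index 0 as the silent option.
; It plays the English voice clip, looks up speaker data and passes stage directions to a StageDirector component created on demand.
; A missing row closes the conversation.
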(fn OpenConversation
  (bind _returnvalue (UserInterface|CreateWidget "/Game/DialogueSystem/UI/WB_Dialogue.WB_Dialogue_C" 0 self))
  (bind _output_get (Variables|Default|SetDialogueWidget _returnvalue))
  (UserInterface|Viewport|AddtoViewport _output_get 0)
  (CallFunction|Dialogue "1"))

(fn CloseConversation
  (bind _stagedirector (Variables|Default|GetStageDirector))
  (Widget|RemovefromParent (Variables|Default|GetDialogueWidget))
  (Utilities|Time|SetGlobalTimeDilation 1.0)
  (if (Utilities|IsValid _stagedirector)
    (Default|TakeDirection _stagedirector "end"))
  (Class|BPIInteractable|ConversationClosed(Message) (Components|GetOwner)))

(fn Dialogue
  (params (blockName :type String))
  (bind _output_get (Variables|Default|SetCurrentBlock blockName))
  ;[0.2083 0.2083 0.2083] Play Line and offer Choice
  (bind (_line _options _speaker _en_sound _stagedirection) (CallFunction|FetchBlockfromDT (Variables|Default|GetTable) (Utilities|String|StringToName _output_get)))
  (bind _output (CallFunction|GetDatabyEnum _speaker))
  (|RunStageDirections _stagedirection
    (:OutputPin
      (Audio|PlaySoundatLocation _en_sound "0, 0, 0" "0, 0, 0" 1.0 1.0 0.0 0 0 0 0)
      (Default|UpdateDialogueText (Variables|Default|GetDialogueWidget) _output _line _options (Variables|Default|GetCurrentBlock) (Variables|Default|GetTable)))))

(fn FetchBlockfromDT
  (params (Table :type Data%20Table%20Object%20Reference) (RowName :type Name))
  (bind _returnvalue (Utilities|GetDataTableRow Table RowName)
    (:then
      (bind _returnvalue_2 (CallFunction|GetLang (.joined_line (Utilities|Struct|BreakS_DT_Dialogue _returnvalue))))
      (|GetOptionsArray Table RowName
        (:Completed
          (return (Utilities|Text|ToText(String) _returnvalue_2) (LocalVariables|GetOptArr) (.speaker (Utilities|Struct|BreakS_DT_Dialogue _returnvalue)) (.en_sound (Utilities|Struct|BreakS_DT_Dialogue _returnvalue)) (.StageDirection (Utilities|Struct|BreakS_DT_Dialogue _returnvalue))))))
    (:RowNotFound
      (CallFunction|CloseConversation))))

(fn GetLang
  (params (SourceString :type String))
  (bind _returnvalue (Utilities|String|ParseIntoArray SourceString "|" false))
  (bind _language (Variables|Default|GetLanguage))
  ;[0.2865 0.2865 0.2865] Continue only if the array has at least one element.
  (if (> (Utilities|Array|Length _returnvalue) _language)
    (LocalVariables|SetOutput (Utilities|Array|Get(acopy) _returnvalue _language)))
  (return (LocalVariables|GetOutput)))

(fn GetDatabyEnum
  (params (InputPin :type Enum_Character%20Enum :default "NewEnumerator0"))
  (Utilities|FlowControl|Sequence
    (:then_0
      (switch Utilities|FlowControl|Switch|SwitchonEnum_Character InputPin
        (:NewEnumerator0
          (LocalVariables|SetIndex 0))
        (:NewEnumerator1
          (LocalVariables|SetIndex 1))
        (:NewEnumerator2
          (LocalVariables|SetIndex 2))
        (:NewEnumerator3
          (LocalVariables|SetIndex 3))))
    (:then_1
      (return (Utilities|Array|Get(acopy) (Variables|Default|GetCharacterData) (LocalVariables|GetIndex))))))