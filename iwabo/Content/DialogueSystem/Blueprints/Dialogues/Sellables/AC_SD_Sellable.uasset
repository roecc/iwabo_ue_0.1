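; Dialogue component for sellables that lets a dialogue direction open a price-setting screen.
; It overrides TakeDirection, calls the parent, then reacts to the "OpenSetPrice" direction.
; It looks up AC_Sellable on the owning actor, passes it into a new WB_SetPrice widget and adds that to the viewport, printing an error if the component is missing.
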(event EventBeginPlay
  (|CallParentFunction) ; This node is disabled and will not be called.\nDrag off pins to build functionality.
)

(event EventTick
  (params (DeltaSeconds :type Float%20%28single-precision%29))
  (|CallParentFunction DeltaSeconds) ; This node is disabled and will not be called.\nDrag off pins to build functionality.
)

(fn TakeDirection
  (params (Direction :type String))
  (bind _returnvalue (Components|GetOwner))
  (bind _returnvalue_2 (Actor|GetComponentbyClass _returnvalue "/Game/BuySellSystem/AC_Sellable.AC_Sellable_C"))
  (|CallParentFunction Direction)
  (if (Utilities|Enum|Equal(Enum) Direction "OpenSetPrice")
    (Utilities|IsValid _returnvalue_2
      (:Is%20Valid
        (bind _returnvalue_3 (UserInterface|CreateWidget "/Game/BuySellSystem/WB_SetPrice.WB_SetPrice_C" 0 _returnvalue_2))
        (UserInterface|Viewport|AddtoViewport _returnvalue_3 0))
      (:Is%20Not%20Valid
        (Development|PrintString "AC_SELLABLE NOT FOUND!!!")))))