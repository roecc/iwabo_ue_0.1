(fn Dialogue
  (|CallParentFunction)
  (switch int (Variables|Default|GetDialogueTreeIndex)
    (:0
      (|Greeting
        (:how%20are%20you%20today?
          (bind _state (CallFunction|AddDialogue "Mary-Ann" "Pretty good, though June is keeping me quite busy." (Utilities|Array|MakeArray "cool.")))
          (switch Utilities|FlowControl|Switch|SwitchonEnum_DialogueState _state
            (:NewEnumerator0
              (CallFunction|ClearDialogueProgress) ; resets conversation
              (CallFunction|CloseConversation))))
        (:Dinner%20done%20yet?
          (bind (_state_2 _optionindex) (CallFunction|AddDialogue "Mary-Ann" "Not quite yet, but you could set the table if you want." (Utilities|Array|MakeArray "sure thing honey." "Nah, I'll wait.")))
          (switch Utilities|FlowControl|Switch|SwitchonEnum_DialogueState _state_2
            (:NewEnumerator0
              (switch int _optionindex
                (:0
                  (bind _state_3 (CallFunction|AddDialogue "Mary-Ann" "Thank you honey!" (Utilities|Array|MakeArray "You're welcome.")))
                  (switch Utilities|FlowControl|Switch|SwitchonEnum_DialogueState _state_3
                    (:NewEnumerator0
                      (Variables|Default|SetDialogueTreeIndex 1))))
                (:1
                  (bind _state_4 (CallFunction|AddDialogue "Mary-Ann" "Very helpful. Thanks." (Utilities|Array|MakeArray "You're welcome.")))
                  (switch Utilities|FlowControl|Switch|SwitchonEnum_DialogueState _state_4
                    (:NewEnumerator0
                      _))))
              (CallFunction|ClearDialogueProgress)
              (CallFunction|CloseConversation))))))
    (:1
      (bind _state_5 (CallFunction|AddDialogue "Mary-Ann" "Thanks again for setting the table" (Utilities|Array|MakeArray "You're Welcome.")))
      (switch Utilities|FlowControl|Switch|SwitchonEnum_DialogueState _state_5
        (:NewEnumerator0
          (CallFunction|ClearDialogueProgress)
          (CallFunction|CloseConversation))))))