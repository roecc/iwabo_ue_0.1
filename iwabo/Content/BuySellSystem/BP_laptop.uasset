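; BP_laptop is an interactable laptop actor that serves as an access point to the buy/sell system.
; On Interact it stores the instigator and opens the buy/sell tab through its ACBuySell component.
; SetInteractableState shows or hides the TxtBuySell prompt, and ConversationClosed notifies the stored instigator through ConversationClosedMessage.
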(event EventBeginPlay)

(event Collision|EventActorBeginOverlap
  (params (OtherActor :type Actor%20Object%20Reference)))

(event EventTick
  (params (DeltaSeconds :type Float%20%28single-precision%29)))

(event EventInteract
  (params (Instigator :type Actor%20Object%20Reference))
  (Variables|Default|SetInteractInstigator Instigator)
  (Default|OpenBuySellTab (Variables|Default|GetAC_BuySell)))

(event EventSetInteractableState
  (params (bCanShowInteract? :type Boolean))
  (bind _txt_buy_sell (Variables|Default|Gettxt_buy_sell))
  (if bCanShowInteract?
    (Rendering|SetVisibility _txt_buy_sell true false)
    (else
      (Rendering|SetVisibility _txt_buy_sell false false))))

(event EventConversationClosed
  (Class|BPIInteractable|ConversationClosed(Message) (Variables|Default|GetInteractInstigator)))

(fn ConstructionScript)