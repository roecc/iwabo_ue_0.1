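; BP_Sellable_Base is the base actor for sellable items in the buy/sell system.
; Interacting opens a conversation through its dialogue component and notifies the instigator when it closes.
; Interact focus toggles custom-depth highlighting on all static meshes and the name text, and the first focus registers the item through ACSellable.
; Update events set the name and estimated price texts and show a post-it while for sale.
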(event Custom|UpdateNameAndPrice
  (params (Name :type Text) (EstPrice :type Integer))
  (Rendering|Components|TextRender|SetText (Variables|Default|Gettxt_name) Name)
  (Rendering|Components|TextRender|SetText (Variables|Default|Gettxt_estPrice) (Utilities|Text|ToText(String) (Utilities|String|BuildString(Integer) "" "$" EstPrice))))

(event Custom|UpdateForSale
  (params (bForSale? :type Boolean))
  (Development|SetHiddeninGame (Variables|Default|Gettmp_postit) (not bForSale?) false))

(event EventInteract
  (params (Instigator :type Actor%20Object%20Reference))
  (Variables|Default|SetInteractInstigator Instigator)
  (Default|OpenConversation (Variables|Default|GetAC_Dialogue_Base)))

(event EventSetInteractableState
  (params (bCanShowInteract? :type Boolean))
  (bind _txt_name (Variables|Default|Gettxt_name))
  (for (_array_element _array_index) (Actor|GetComponentsByClass "/Script/Engine.StaticMeshComponent")
    (Development|PrintString (Utilities|String|ToString(Integer) _array_index))
    (Rendering|SetRenderCustomDepth _array_element bCanShowInteract?)
    (Development|PrintString "highlight"))
  (if bCanShowInteract?
    (Development|SetHiddeninGame _txt_name false true)
    (Utilities|FlowControl|DoOnce false
      (:Completed
        (Default|AddItemtoList (Variables|Default|GetAC_Sellable))))
    (else
      (Development|SetHiddeninGame _txt_name true true))))

(event EventConversationClosed
  (Class|BPIInteractable|ConversationClosed(Message) (Variables|Default|GetInteractInstigator)))

(fn ConstructionScript)