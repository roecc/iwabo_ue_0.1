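; AC_SD_Box handles string directions for the Dad Box interactable, opening and closing the dad's note on screen.
; TakeDirection calls the parent implementation, then on OpenLetter creates a WB_DadNote widget, stores it in LetterRef and adds it to the viewport.
; On CloseLetter it removes that stored widget, or prints a warning if the reference is invalid.
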(event EventBeginPlay)

(event EventTick
  (params (DeltaSeconds :type Float%20%28single-precision%29)))

(fn TakeDirection
  (params (Direction :type String))
  (|CallParentFunction Direction)
  (if (Utilities|Enum|Equal(Enum) Direction "OpenLetter")
    (bind _returnvalue (UserInterface|CreateWidget "/Game/Interactables/DadBox/WB_DadNote.WB_DadNote_C"))
    (bind _output_get (Variables|Default|SetLetterRef _returnvalue))
    (UserInterface|Viewport|AddtoViewport _output_get 0)
    (elif (Utilities|Enum|Equal(Enum) Direction "CloseLetter")
      (Utilities|IsValid (Variables|Default|GetLetterRef)
        (:Is%20Valid
          (Widget|RemovefromParent (Variables|Default|GetLetterRef)))
        (:Is%20Not%20Valid
          (Development|PrintString "No Letter Ref!"))))))