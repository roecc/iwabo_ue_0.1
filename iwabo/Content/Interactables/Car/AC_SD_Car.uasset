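; Actor component for the interactable car that handles a "Teleport" direction, simulating a drive to another location.
; It overrides TakeDirection, calls the parent, then triggers the Teleport event on a matching direction.
; Teleport plays the drive sound at the car, waits briefly, moves the interact instigator to TeleportTarget's position and rotation, then sets the Sun light's intensity to Brightness.
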(event Custom|Teleport
  (bind _teleporttarget (Variables|Default|GetTeleportTarget))
  (bind _returnvalue (Transformation|GetActorTransform _teleporttarget))
  (Audio|PlaySoundatLocation "/Game/tmp_assets/driveCar.driveCar" (.location (Transformation|GetActorTransform (Components|GetOwner))) "0, 0, 0" 1.0 1.0 0.0 0 0 0 0)
  (Utilities|FlowControl|Delay 2.0)
  ;[0.1979 0.1979 0.1979] Teleport Player
  (bind _asbp_interactable_car (Utilities|Casting|CastToBP_Interactable_Car (Components|GetOwner)))
  (Transformation|SetWorldTransform (Variables|/Script/Engine.Actor|GetRootComponent (Variables|/Game/Interactables/BP_Interactable_Base.BP_Interactable_Base_C|GetInteractInstigator _asbp_interactable_car)) (Math|Transform|MakeTransform (.location _returnvalue) (.rotation _returnvalue) "1.000000,1.000000,1.000000") false true)
  ;[0.1979 0.1979 0.1979] Set Sun
  (Rendering|Components|Light|SetIntensity (Variables|/Script/Engine.Light|GetLightComponent (Variables|Default|GetSun)) (Variables|Default|GetBrightness)))

(event EventBeginPlay)

(event EventTick
  (params (DeltaSeconds :type Float%20%28single-precision%29)))

(fn TakeDirection
  (params (Direction :type String))
  (|CallParentFunction Direction)
  (if (Utilities|Enum|Equal(Enum) Direction "Teleport")
    (CallFunction|Teleport)))