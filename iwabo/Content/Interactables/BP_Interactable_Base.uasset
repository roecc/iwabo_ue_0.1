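; Base interactable actor Blueprint that provides a name label, outline highlighting and optional conversation on interaction.
; Interact stores the instigator and opens the dialogue component's conversation when flagged as a conversation, then ConversationClosed notifies that instigator.
; Outlines use custom depth on all static meshes: interactable state toggles rendering, while active state switches the stencil value and shows or hides the name text.
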(event Custom|UpdateName
  (params (Name :type Text) (EstPrice :type Integer))
  (Rendering|Components|TextRender|SetText (Variables|Default|Gettxt_name) Name))

(event EventSetActiveState
  (params (bIsActive? :type Boolean))
  (bind _txt_name (Variables|Default|Gettxt_name))
  ;[0.09375 0.09375 0.09375] Switch active/available Outline and Name
  (for _array_element (Actor|GetComponentsByClass "/Script/Engine.StaticMeshComponent")
    (if bIsActive?
      (Rendering|SetCustomDepthStencilValue _array_element 0)
      (else
        (Rendering|SetCustomDepthStencilValue _array_element 1))))
  (if bIsActive?
    (Development|SetHiddeninGame _txt_name false true)
    (else
      (Development|SetHiddeninGame _txt_name true true))))

(event EventInteract
  (params (Instigator :type Actor%20Object%20Reference))
  (Variables|Default|SetInteractInstigator Instigator)
  (if (Variables|Default|GetbIsConversation?)
    (Default|OpenConversation (Variables|Default|GetAC_Dialogue_Base))))

(event EventSetInteractableState
  (params (bCanShowInteract? :type Boolean))
  ;[0.125 0.125 0.125] Set Outline
  (for _array_element (Actor|GetComponentsByClass "/Script/Engine.StaticMeshComponent")
    (Rendering|SetRenderCustomDepth _array_element bCanShowInteract?)))

(event EventConversationClosed
  (Class|BPIInteractable|ConversationClosed(Message) (Variables|Default|GetInteractInstigator)))

(fn ConstructionScript)