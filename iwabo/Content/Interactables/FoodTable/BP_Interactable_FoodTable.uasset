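; BP_Interactable_FoodTable is an interactable food table that holds an interaction open until the player moves.
; Interact stores the instigator, enables input on the table for player 0, then switches to game-only input mode after a short delay.
; The IA_Move input action triggers ConversationClosed, which disables the table's input and sends ConversationClosedMessage to the stored instigator.
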(event Input|EnhancedActionEvents|EnhancedInputActionIA_Move
  (params (ActionValue :type Vector%202D%20Structure) (ElapsedSeconds :type Float%20%28double-precision%29) (TriggeredSeconds :type Float%20%28double-precision%29) (InputAction :type Input%20Action%20Object%20Reference :default "/Game/ThirdPerson/Input/Actions/IA_Move.IA_Move"))
  (CallFunction|ConversationClosed))

(event EventBeginPlay)

(event Collision|EventActorBeginOverlap
  (params (OtherActor :type Actor%20Object%20Reference)))

(event EventTick
  (params (DeltaSeconds :type Float%20%28single-precision%29)))

(event EventInteract
  (params (Instigator :type Actor%20Object%20Reference))
  (bind _output_get (Variables|Default|SetInteractInstigator Instigator))
  (Input|EnableInput (Game|GetPlayerController 0))
  (Utilities|FlowControl|Delay 0.2)
  (Input|SetInputModeGameOnly (Game|GetPlayerController 0) false))

(event EventConversationClosed
  (Input|DisableInput (Game|GetPlayerController 0))
  (Class|BPIInteractable|ConversationClosed(Message) (Variables|Default|GetInteractInstigator)))

(fn ConstructionScript
  (|CallParentFunction))