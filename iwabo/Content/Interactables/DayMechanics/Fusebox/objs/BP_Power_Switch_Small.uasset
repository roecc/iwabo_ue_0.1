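; A small clickable power switch for the fusebox mechanic that toggles power through a room manager.
; Clicking its box drives a FlipFlop that tilts the switch pivot 45 degrees in relative pitch, alternating direction.
; Each flip sends the matching power-up or power-down message to the room manager, or prints an error if none is assigned.
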(event OnClicked(Box)
  (params (TouchedComponent :type Primitive%20Component%20Object%20Reference) (ButtonPressed :type Key%20Structure :default "None"))
  (bind _roommanager (Variables|Default|GetRoomManager))
  (bind _roommanager_2 (Variables|Default|GetRoomManager))
  (bind _switchpivot (Variables|Default|GetSwitchPivot))
  (bind _relativerotation (Variables|/Script/Engine.SceneComponent|GetRelativeRotation _switchpivot))
  (Utilities|FlowControl|FlipFlop
    (:A
      (Transformation|SetRelativeRotation _switchpivot (Math|Rotator|MakeRotator (.roll _relativerotation) (+ (.pitch _relativerotation) -45.0) (.yaw _relativerotation)) false false)
      (Utilities|IsValid _roommanager_2
        (:Is%20Valid
          (Class|BPIPowerable|PowerUp(Message) _roommanager_2))
        (:Is%20Not%20Valid
          (Development|PrintString "Error, Power_RoomManager not assigned."))))
    (:B
      (Transformation|SetRelativeRotation _switchpivot (Math|Rotator|MakeRotator (.roll _relativerotation) (+ (.pitch _relativerotation) 45.0) (.yaw _relativerotation)) false false)
      (Utilities|IsValid _roommanager
        (:Is%20Valid
          (Class|BPIPowerable|PowerDown(Message) _roommanager))
        (:Is%20Not%20Valid
          (Development|PrintString "Error, Power_RoomManager not assigned."))))))

(event EventBeginPlay)

(event Collision|EventActorBeginOverlap
  (params (OtherActor :type Actor%20Object%20Reference)))

(event EventTick
  (params (DeltaSeconds :type Float%20%28single-precision%29)))

(fn ConstructionScript)