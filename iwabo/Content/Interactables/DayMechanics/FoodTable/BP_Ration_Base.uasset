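; BP_Ration_Base is a base food-table ration actor that can be picked up and moved with the mouse.
; Clicking its Box flips the Clicked state through a FlipFlop, toggling follow mode on and off.
; While Clicked, Tick line-traces the Visibility channel along the deprojected cursor ray and sweeps the actor to the hit location.
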(event OnClicked(Box)
  (params (TouchedComponent :type Primitive%20Component%20Object%20Reference) (ButtonPressed :type Key%20Structure :default "None"))
  (bind _isa (Utilities|FlowControl|FlipFlop)
    (:A
      _)
    (:B
      _))
  (bind _output_get (Variables|Default|SetbClicked? _isa)))

(event EventBeginPlay)

(event Collision|EventActorBeginOverlap
  (params (OtherActor :type Actor%20Object%20Reference)))

(event EventTick
  (params (DeltaSeconds :type Float%20%28single-precision%29))
  (bind _returnvalue (Game|GetPlayerController 0))
  (bind (_worldlocation _worlddirection) (Game|Player|ConvertMouseLocationToWorldSpace _returnvalue))
  (if (stale OnClicked(Box) _output_get)
    (bind (_outhit _returnvalue_2) (Collision|LineTraceByChannel _worldlocation (+ _worldlocation (* _worlddirection 1e+04)) "TraceTypeQuery1" false 0 "None"))
    (if _returnvalue_2
      (Transformation|SetActorLocation (.Location (Collision|BreakHitResult _outhit)) true false))))

(fn ConstructionScript)