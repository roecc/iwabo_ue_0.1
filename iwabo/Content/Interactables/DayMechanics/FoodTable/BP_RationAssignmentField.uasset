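; Food table zone for one named character that tracks the rations placed inside it.
; After a one-second delay on BeginPlay it caches that character's mood column from the game instance's mood widget by CharID.
; Box begin and end overlaps add or remove rations from the local list, refresh the column's food display and adjust the game instance's per-type assigned counts.
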(event OnComponentBeginOverlap(Box)
  (params (OverlappedComponent :type Primitive%20Component%20Object%20Reference) (OtherActor :type Actor%20Object%20Reference) (OtherComp :type Primitive%20Component%20Object%20Reference) (OtherBodyIndex :type Integer) (bFromSweep :type Boolean) (SweepResult :type Hit%20Result%20Structure%20%28by%20ref%29))
  (bind _asbp_ration_base (Utilities|Casting|CastToBP_Ration_Base OtherActor))
  (if (not (Utilities|Array|ContainsItem (Variables|Default|GetAssignedRations) _asbp_ration_base))
    (Utilities|Array|Add (Variables|Default|GetAssignedRations) _asbp_ration_base)
    (Default|UpdateFood (Variables|Default|GetMoodColumn) self)
    (bind _asbp_game_instance (Utilities|Casting|CastToBP_GameInstance (Game|GetGameInstance)))
    (Utilities|Map|Add (Variables|/Game/GameManagement/BP_GameInstance.BP_GameInstance_C|GetAssignedRations _asbp_game_instance) (Variables|/Game/Interactables/DayMechanics/FoodTable/BP_Ration_Base.BP_Ration_Base_C|GetRationType _asbp_ration_base) (+ (.Value (Utilities|Map|Find (Variables|/Game/GameManagement/BP_GameInstance.BP_GameInstance_C|GetAssignedRations _asbp_game_instance) (Variables|/Game/Interactables/DayMechanics/FoodTable/BP_Ration_Base.BP_Ration_Base_C|GetRationType _asbp_ration_base))) 1))))

(event OnComponentEndOverlap(Box)
  (params (OverlappedComponent :type Primitive%20Component%20Object%20Reference) (OtherActor :type Actor%20Object%20Reference) (OtherComp :type Primitive%20Component%20Object%20Reference) (OtherBodyIndex :type Integer))
  (bind _assignedrations (Variables|Default|GetAssignedRations))
  (bind _asbp_ration_base (Utilities|Casting|CastToBP_Ration_Base OtherActor))
  (if (Utilities|Array|ContainsItem _assignedrations _asbp_ration_base)
    (Utilities|Array|RemoveItem _assignedrations _asbp_ration_base)
    (Default|UpdateFood (Variables|Default|GetMoodColumn) self)
    (bind _asbp_game_instance (Utilities|Casting|CastToBP_GameInstance (Game|GetGameInstance)))
    (Utilities|Map|Add (Variables|/Game/GameManagement/BP_GameInstance.BP_GameInstance_C|GetAssignedRations _asbp_game_instance) (Variables|/Game/Interactables/DayMechanics/FoodTable/BP_Ration_Base.BP_Ration_Base_C|GetRationType _asbp_ration_base) (+ (.Value (Utilities|Map|Find (Variables|/Game/GameManagement/BP_GameInstance.BP_GameInstance_C|GetAssignedRations _asbp_game_instance) (Variables|/Game/Interactables/DayMechanics/FoodTable/BP_Ration_Base.BP_Ration_Base_C|GetRationType _asbp_ration_base))) -1))))

(event EventBeginPlay
  (Rendering|Components|TextRender|SetText (Variables|Default|Gettxt_Name) (Variables|Default|GetName))
  (Utilities|FlowControl|Delay 1.0)
  ;[1 1 1] get mood column ref
  (bind _asbp_game_instance (Utilities|Casting|CastToBP_GameInstance (Game|GetGameInstance)))
  (Variables|Default|SetMoodColumn (Utilities|Array|Get(acopy) (Variables|/Game/Debug/Mood/Debug_WB_Mood_Main.Debug_WB_Mood_Main_C|GetColumns (Variables|/Game/GameManagement/BP_GameInstance.BP_GameInstance_C|GetWB_Mood _asbp_game_instance)) (Variables|Default|GetCharID))))

(fn ConstructionScript)