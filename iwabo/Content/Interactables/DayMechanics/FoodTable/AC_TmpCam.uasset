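; AC_TmpCam is a component that temporarily switches the game camera, filed with the food table day-mechanic interactables.
; SwitchToTmp takes the third-person character and, if its current camera is not already NewCamera, saves that camera as OldCamera and switches to NewCamera.
; SwitchBack restores the saved camera.
; Both switches go through SwitchCam on BP_GameInstance.
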(event Custom|SwitchToTmp
  (params (Col :type Object%20Object%20Reference))
  (bind _asbp_third_person_character (Utilities|Casting|CastToBP_ThirdPersonCharacter Col))
  (if (not (== (Variables|/Game/ThirdPerson/Blueprints/BP_ThirdPersonCharacter.BP_ThirdPersonCharacter_C|GetCurrentCam _asbp_third_person_character) (Variables|Default|GetNewCamera)))
    (Variables|Default|SetOldCamera (Variables|/Game/ThirdPerson/Blueprints/BP_ThirdPersonCharacter.BP_ThirdPersonCharacter_C|GetCurrentCam _asbp_third_person_character))
    (bind _asbp_game_instance (Utilities|Casting|CastToBP_GameInstance (Game|GetGameInstance)))
    (Default|SwitchCam _asbp_game_instance (Variables|Default|GetNewCamera))))

(event Custom|SwitchBack
  (bind _asbp_game_instance (Utilities|Casting|CastToBP_GameInstance (Game|GetGameInstance)))
  (Default|SwitchCam _asbp_game_instance (Variables|Default|GetOldCamera)))