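; BP_Interactable_Bed is the bed interactable that ends the current turn, presented as the end of a day.
; On interaction it creates and adds a WB_EndDay widget once, calls EndTurn on BP_GameInstance, then refreshes the widget's text and starts a new turn on FoodTable.
; After a short delay it calls ConversationClosed and shows the day text; the timed collapse of that text is disconnected.
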(event EventInteract
  (params (Instigator :type Actor%20Object%20Reference))
  (Variables|Default|SetInteractInstigator Instigator)
  (Utilities|FlowControl|Sequence
    (:then_0
      (Utilities|FlowControl|DoOnce false
        (:Completed
          (bind _returnvalue (UserInterface|CreateWidget "/Game/Interactables/DayMechanics/Bed/WB_EndDay.WB_EndDay_C"))
          (bind _output_get (Variables|Default|SetDayText _returnvalue))
          (UserInterface|Viewport|AddtoViewport _output_get 0))))
    (:then_1
      (bind _asbp_game_instance (Utilities|Casting|CastToBP_GameInstance (Game|GetGameInstance)))
      (Default|EndTurn _asbp_game_instance)
      (Default|UpdateText (Variables|Default|GetDayText)))
    (:then_2
      (Default|NewTurn (Variables|Default|GetFoodTable)))
    (:then_3
      (Utilities|FlowControl|Delay 0.1)
      (CallFunction|ConversationClosed)
      (Widget|SetVisibility (Variables|Default|GetDayText) "HitTestInvisible"))))

(fn ConstructionScript
  (|CallParentFunction))